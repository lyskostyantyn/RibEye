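; BP_Run is a trigger actor with a floating text label that starts a throwable scenario, apparently for testing or demonstrating enemy search behavior.
; The label shows configurable text and turns with the player camera each tick.
; The player's first box overlap with a valid Throwable runs its countdown and teleports the player to it.
; A positive MaxSearcherCount then overrides that setting on every BP_EnemyBase's social component, preserving the other settings.
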(event `self.ReceiveBeginPlay`
  (`TextRenderComponent.K2_SetText` (`self.TextRender`) (`self.TextToShow`)))

(event `self.ReceiveTick`
  (params (DeltaSeconds :type "Float (single-precision)"))
  (bind _textrender (`self.TextRender`))
  (`SceneComponent.K2_SetWorldRotation` _textrender (`PlayerCameraManager.GetCameraRotation` (`GameplayStatics.GetPlayerCameraManager` 0)) false false)
  (`SceneComponent.K2_AddLocalRotation` _textrender (struct :`Yaw` 180.0) false false))

(event `self.Box.OnComponentBeginOverlap`
  (params (OverlappedComponent :type "PrimitiveComponent Object Reference") (OtherActor :type "Actor Object Reference") (OtherComp :type "PrimitiveComponent Object Reference") (OtherBodyIndex :type Integer) (bFromSweep :type Boolean) (SweepResult :type "HitResult Structure (by ref)"))
  (bind _throwable (`self.Throwable`))
  (if (== OtherActor (`GameplayStatics.GetPlayerPawn` 0))
    (`/Engine/EditorBlueprintResources/StandardMacros.IsValid` _throwable
      (:`Is Valid`
        (`/Engine/EditorBlueprintResources/StandardMacros.DoOnce` false
          (:`Completed`
            (`/Game/BP_ThrowableStatic.RunCountdown` _throwable)
            (`self.K2_TeleportTo` :`self` OtherActor :`DestLocation` (`self.K2_GetActorLocation` (`self.Throwable`)))
            (if (> (`self.MaxSearcherCount`) 0)
              (bind _outactors (`GameplayStatics.GetAllActorsOfClass` "/Game/AI/BP_EnemyBase.BP_EnemyBase_C"))
              (for _array_element _outactors
                (bind _returnvalue (`self.GetComponentByClass` _array_element "/Game/AI/Components/BP_SocialComponent.BP_SocialComponent_C"))
                (`/Engine/EditorBlueprintResources/StandardMacros.IsValid` _returnvalue
                  (:`Is Valid`
                    (bind (_settings_maxinvestigators _settings_resolvewholegroupofai _settings_dialoguestoignore) (break `SocialSettings` (`SocialComponent.Settings` _returnvalue)))
                    (set `SocialComponent.Settings` (make `SocialSettings` (`self.MaxSearcherCount`) _settings_resolvewholegroupofai _settings_dialoguestoignore) _returnvalue)))))))))))

(fn `UserConstructionScript`)