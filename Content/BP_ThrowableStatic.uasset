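; Throwable child Blueprint that acts as a timed noise maker, turning off activate-on-hit at BeginPlay.
; RunCountdown shows a text label and re-arms a DoOnce, which Tick fires to start a delay ending in a noise event at the actor's location.
; Tick also decrements the displayed time, turns the label to face the camera and optionally draws the noise radius as a debug sphere.
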(event `self.ReceiveBeginPlay`
  (`parent.ReceiveBeginPlay`)
  (set `self.ActiveOnHit` false))

(event `RunCountdown`
  (set `self.ExplosionTimeRemaining` (`self.Auto Explosion Time`))
  (`SceneComponent.SetVisibility` (`self.TextRender`) true false)
  (goto _label :!via `Reset`))

(event `self.ReceiveTick`
  (params (DeltaSeconds :type "Float (single-precision)"))
  (bind _textrender (`self.TextRender`))
  (`|ExecutionSequence`
    (:`then_0`
      (if (> (`self.ExplosionTimeRemaining`) 0.0)
        (`|ExecutionSequence`
          (:`then_0`
            (`/Engine/EditorBlueprintResources/StandardMacros.DoOnce` true :!label _label
              (:`Completed`
                (`KismetSystemLibrary.Delay` (`self.Auto Explosion Time`))
                (`AISense_Hearing.ReportNoiseEvent` (`self.K2_GetActorLocation`) 1.0 self (`self.Max Range`))
                (`SceneComponent.SetVisibility` (`self.TextRender`) false false))))
          (:`then_1`
            (set `self.ExplosionTimeRemaining` (- (`self.ExplosionTimeRemaining`) DeltaSeconds)))
          (:`then_2`
            (`TextRenderComponent.K2_SetText` (`self.TextRender`) (`KismetTextLibrary.Conv_DoubleToText` (`self.ExplosionTimeRemaining`) "HalfToEven"))
            (`SceneComponent.K2_SetWorldRotation` _textrender (`PlayerCameraManager.GetCameraRotation` (`GameplayStatics.GetPlayerCameraManager` 0)) false false)
            (`SceneComponent.K2_AddLocalRotation` _textrender (struct :`Yaw` 180.0) false false)))))
    (:`then_1`
      (if (`self.Draw Debug`)
        (`KismetSystemLibrary.DrawDebugSphere` (`self.K2_GetActorLocation`) (`self.Max Range`) 12 (struct :`R` 1.0 :`G` 0.839216 :`A` 1.0))))))

(fn `UserConstructionScript`
  (`parent.UserConstructionScript`))