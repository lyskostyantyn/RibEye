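; AI component for BP_EnemyBase that manages social identity and decides whether others may join its investigation group.
; On BeginPlay it sets up an ID and writes it to the owner's ID text, which Tick turns toward the player or debug camera.
; Membership checks compare group size against the investigator limit, returning reply types for reject, join, join-last or partial join, split by single or multiple, with an accepted count.
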(event `self.ReceiveBeginPlay`
  ; Set ID
  (`self.SetupID`)
  (bind _asbp_enemy_base (cast `/Game/AI/BP_EnemyBase` (`self.GetOwner`)))
  (set `self.Owner` _asbp_enemy_base)
  (`TextRenderComponent.K2_SetText` (`/Game/AI/BP_EnemyBase.ID` (`self.Owner`)) (`KismetTextLibrary.Conv_StringToText` (`KismetStringLibrary.Concat_StrStr` (`self.GetTextID`) (`KismetStringLibrary.Concat_StrStr` " AI " (`KismetStringLibrary.Conv_IntToString` (`self.GetID`)))))))

(event `self.ReceiveTick`
  (params (DeltaSeconds :type "Float (single-precision)"))
  (bind _id (`/Game/AI/BP_EnemyBase.ID` (`self.Owner`)))
  ; DIsplay Dialog Subtitle
  (bind _asdebug_camera_controller (cast `DebugCameraController` (`GameplayStatics.GetPlayerController` 0))
    (:`then`
      (set `self.CameraToUse` (`PlayerController.PlayerCameraManager` _asdebug_camera_controller)))
    (:`CastFailed`
      (set `self.CameraToUse` (`GameplayStatics.GetPlayerCameraManager` 0))))
  (`SceneComponent.K2_SetWorldRotation` _id (`PlayerCameraManager.GetCameraRotation` (`self.CameraToUse`)) false false)
  (`SceneComponent.K2_AddLocalRotation` _id (struct :`Yaw` 180.0) false false))

(fn `CanAcceptNewMembers`
  (params (NewMembers :type Integer) (GroupType :type "EGroupType Enum" :default "PATROL"))
  (returns (ReplyType :type "EJoinReplyType Enum") (Multiple :type Boolean) (CountToAccept :type Integer))
  (locals (IsMultiple :type Boolean))
  (bind _returnvalue (`self.GetSocialGroupSize`))
  (bind _settings_maxinvestigators (break `SocialSettings` (`self.Settings`)))
  (bind _returnvalue_2 (- _settings_maxinvestigators _returnvalue))
  (set `local.IsMultiple` (> _returnvalue 1))
  (switch `EGroupType` GroupType
    (:`INVESTIGATE`
      (if (== _returnvalue_2 0)
        (return "REJECT" (`local.IsMultiple`) 0)
        (elif (== _returnvalue_2 (`local.NewMembers`))
          (if (> (`local.NewMembers`) 1)
            (bind _result (`/Engine/EditorBlueprintResources/StandardMacros.NegateInt` (`local.NewMembers`))
              (:`  `
                (return "CAN_JOIN_LAST_MULT" (`local.IsMultiple`) _result)))
            (else
              (bind _result_2 (`/Engine/EditorBlueprintResources/StandardMacros.NegateInt` (`local.NewMembers`))
                (:`  `
                  (return "CAN_JOIN_LAST_SINGLE" (`local.IsMultiple`) _result_2)))))
          (elif (> _returnvalue_2 (`local.NewMembers`))
            (if (> (`local.NewMembers`) 1)
              (return "CAN_JOIN_MULT" (`local.IsMultiple`) (`local.NewMembers`))
              (else
                (return "CAN_JOIN_SINGLE" (`local.IsMultiple`) (`local.NewMembers`))))
            (else
              (bind _result_3 (`/Engine/EditorBlueprintResources/StandardMacros.NegateInt` (`local.NewMembers`))
                (:`  `
                  (return "CAN_JOIN_SOME_MULT" (`local.IsMultiple`) _result_3))))))))))

(fn `CanAddNewToInvestigation`
  (returns (CanAdd :type Boolean) (Multiple :type Boolean))
  (bind _returnvalue (`self.GetSocialGroupSize`))
  (bind _settings_maxinvestigators (break `SocialSettings` (`self.Settings`)))
  (return (and (< _returnvalue _settings_maxinvestigators) (not (`self.RejectEverything`))) (> _returnvalue 1)))