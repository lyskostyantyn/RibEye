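; Base enemy AI character that reacts to heard enemies, allies and threats with investigation, alert states and spoken dialogue.
; Knowledge, perception and social events write threat and investigation keys to the Blackboard and manage investigation groups.
; Alert changes set walk speed and an overhead icon.
; Seeing an ally change state picks a line type from both alert states, then starts a dialogue or queues to join an uninterruptible one.
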(event `self.ReceiveBeginPlay`
  (if (`self.IsStaticPatrolling`)
    (`BlackboardComponent.SetValueAsVector` (`AIBlueprintHelperLibrary.GetBlackboard` null) "StaticPatrollingPosition" (`self.K2_GetActorLocation`))
    (`BlackboardComponent.SetValueAsRotator` (`AIBlueprintHelperLibrary.GetBlackboard` null) "StaticPatrollingRotation" (`self.K2_GetActorRotation`))))

(event `self.ReceiveTick`
  (params (DeltaSeconds :type "Float (single-precision)")))

(event `self.Dialogue.OnReplyRequested`
  (params (DialogueID :type Integer))
  ; DialogueCompoenent
  (`/Game/AI/Components/BP_DialogueComponent.OnReplyOnDialogue` (`self.Dialogue`) DialogueID))

(event `self.BP_Social.OnAlertnessChanged`
  (params (AlertState :type "EAlert Enum" :default "PASSIVE"))
  ; Social component
  (`self.OnAlertStateChanged` AlertState))

(event `self.BP_Social.OnSawAllyChangedState`
  (params (Ally :type "Actor Object Reference") (AlertState :type "EAlert Enum" :default "PASSIVE"))
  ; Social component
  (`self.OnSawAllyChangedState` Ally AlertState))

(event `self.Knowledge.OnTargetSelected`
  (params (Target :type "Actor Object Reference"))
  ; Knowledge Component
  (`BlackboardComponent.SetValueAsObject` (`AIBlueprintHelperLibrary.GetBlackboard` null) "BestThreat" Target))

(event `self.Knowledge.OnLastTargetLost`
  (params (Target :type "Actor Object Reference") (LastKnownData :type "LastKnownData Structure (by ref)"))
  ; Knowledge Component
  (`BlackboardComponent.ClearValue` (`AIBlueprintHelperLibrary.GetBlackboard` null) "BestThreat")
  (`BlackboardComponent.SetValueAsBool` (`AIBlueprintHelperLibrary.GetBlackboard` null) "IsSearchAggressive" true)
  (`BlackboardComponent.SetValueAsVector` (`AIBlueprintHelperLibrary.GetBlackboard` null) "InvestigatePosition" LastKnownData_LastKnownPosition))

(fn `DebugOutput`
  (params (Text :type String) (Params :type "Array of String"))
  (locals (StringToOutput :type String))
  (set `local.StringToOutput` Text)
  (for (_array_element _array_index) Params
    (set `local.StringToOutput` (`KismetStringLibrary.Replace` (`local.StringToOutput`) (`KismetStringLibrary.Concat_StrStr` "%" (`KismetStringLibrary.Conv_IntToString` _array_index)) _array_element)))
  (`KismetSystemLibrary.PrintString` (`KismetStringLibrary.Concat_StrStr` (`KismetStringLibrary.Concat_StrStr` "AI " (`KismetStringLibrary.Conv_IntToString` (`SocialComponent.GetID` (`self.BP_Social`))) ":") (`local.StringToOutput`))))

(fn `GetInvestigationPriority`
  (params (Actor :type "Actor Object Reference"))
  (returns (Priority :type "Float (double-precision)"))
  (bind _returnvalue (`AIBlueprintHelperLibrary.GetBlackboard` Actor))
  (bind _returnvalue_2 (`AIBlueprintHelperLibrary.GetCurrentPath` (`AIBlueprintHelperLibrary.GetAIController` Actor)))
  (`/Engine/EditorBlueprintResources/StandardMacros.IsValid` _returnvalue_2
    (:`Is Valid`
      (return (/ 100.0 (`NavigationPath.GetPathLength` _returnvalue_2))))
    (:`Is Not Valid`
      (`/Engine/EditorBlueprintResources/StandardMacros.IsValid` (`BlackboardComponent.GetValueAsObject` _returnvalue "InvestigationPosition")
        (:`Is Valid`
          (return (/ 100.0 (`KismetMathLibrary.VSize` (- (`self.K2_GetActorLocation` Actor) (`BlackboardComponent.GetValueAsVector` _returnvalue "InvestigationPosition"))))))
        (:`Is Not Valid`
          (return 0.0))))))

(fn `OnAlertStateChanged`
  (params (AlertState :type "EAlert Enum" :default "PASSIVE"))
  (switch `EAlert` AlertState
    (:`PASSIVE`
      _)
    (:`INVESTIGATE`
      (`SocialComponent.RemoveActorFromGroup` (`self.BP_Social`) self (cast `EGroupType` 0)))
    (:`AGGRESSIVE_INVESTIGATE`
      _)
    (:`AGGRESSIVE`
      _))
  ; SetNewAlertState
  (if (== AlertState 0)
    (`SceneComponent.SetHiddenInGame` (`self.OverheadIcon`) true false)
    (set `CharacterMovementComponent.MaxWalkSpeed` 200.0 (`self.CharacterMovement`))
    (else
      (`SceneComponent.SetHiddenInGame` (`self.OverheadIcon`) false false)
      (switch `EAlert` AlertState
        (:`INVESTIGATE`
          (`BillboardComponent.SetSprite` (`self.OverheadIcon`) "/Game/HUD/AlertIcons/caution.caution")
          (set `CharacterMovementComponent.MaxWalkSpeed` 300.0 (`self.CharacterMovement`)))
        (:`AGGRESSIVE_INVESTIGATE`
          (`BillboardComponent.SetSprite` (`self.OverheadIcon`) "/Game/HUD/AlertIcons/warning.warning")
          (set `CharacterMovementComponent.MaxWalkSpeed` 400.0 (`self.CharacterMovement`) :!label _label))
        (:`AGGRESSIVE`
          (`BillboardComponent.SetSprite` (`self.OverheadIcon`) "/Game/HUD/AlertIcons/alarm.alarm")
          (goto _label))))))

(fn `OnAllyHeard`
  (params (Ally :type "Actor Object Reference") (Stimulus :type "AIStimulus Structure"))
  (bind _returnvalue (`self.GetComponentByClass` "/Game/AI/Components/BP_DialogueComponent.BP_DialogueComponent_C"))
  (bind _returnvalue_2 (`self.GetComponentByClass` (`GameplayStatics.GetGameState`) "/Script/RibEye.DialogueManager"))
  (if (== Ally self)
    (`self.DebugOutput` "")
    (elif (== Stimulus_Tag "Dialogue")
      (`/Engine/EditorBlueprintResources/StandardMacros.IsValid` _returnvalue
        (:`Is Valid`
          (`/Engine/EditorBlueprintResources/StandardMacros.IsValid` _returnvalue_2
            (:`Is Valid`
              (bind _returnvalue_3 (`DialogueComponent.GetLastDialogueID` _returnvalue))
              (bind (_returnvalue_participants _returnvalue_dialogue) (break `DialogueData` (`DialogueManager.GetDialogueByID` _returnvalue_2 _returnvalue_3)))
              (bind _returnvalue_4 (`KismetArrayLibrary.Array_LastIndex` _returnvalue_dialogue))
              (if (>= _returnvalue_4 0)
                (bind (_output_speaker _output_replier _output_lineentry) (break `DialogueLine` (`|GetArrayItem` _returnvalue_dialogue _returnvalue_4)))
                (bind _returnvalue_5 (`DialogueComponent.OnDialogueHeard` (`self.Dialogue`) _returnvalue_3 (make `DialogueLine` _output_speaker _output_replier _output_lineentry)))
                (bind (_linedata _additionaldata) (break `LineEntry` _output_lineentry))
                (`/Game/AI/Components/BP_DialogueComponent.ProcessHeardLine` (`self.Dialogue`) _output_speaker _output_replier (break `LineData` _linedata) _additionaldata _returnvalue_5 _returnvalue_3)))))))))

(fn `OnEnemyHeard`
  (params (Instigator :type "Actor Object Reference") (Stimulus :type "AIStimulus Structure"))
  (`SocialComponent.AddActorToGroup` (`self.BP_Social`) self "INVESTIGATE")
  (`BlackboardComponent.SetValueAsVector` (`AIBlueprintHelperLibrary.GetBlackboard` null) "InvestigatePosition" Stimulus_StimulusLocation)
  (if (== (`SocialComponent.AlertState` (`self.BP_Social`)) (`KismetMathLibrary.Conv_ByteToInt` (enumliteral `EAlert` "PASSIVE")))
    (bind _canplay (`/Game/AI/Components/BP_DialogueComponent.CanPlayADialogue` (`self.Dialogue`) "INVESTIGATE" -1))
    (if _canplay
      (`DialogueManager.MakeABark` (`DialogueComponent.DialogueManager` (`self.Dialogue`)) Instigator (make `BarkSpeakerData` self "SURPRISED" (`/Game/AI/Components/BP_DialogueComponent.GetSpeakPriority` (`self.Dialogue`) false Stimulus_StimulusLocation "INVALID"))))))

(fn `OnJoinInvestigation`
  (params (Ally :type "Actor Object Reference"))
  (bind _returnvalue (`self.GetComponentByClass` Ally "/Script/RibEye.SocialComponent"))
  (`/Engine/EditorBlueprintResources/StandardMacros.IsValid` Ally
    (:`Is Valid`
      (`/Engine/EditorBlueprintResources/StandardMacros.IsValid` _returnvalue
        (:`Is Valid`
          (`SocialComponent.AddActorToGroup` _returnvalue self "INVESTIGATE")
          (bind _returnvalue_2 (`SocialComponent.GetGroupMembers` _returnvalue "INVESTIGATE"))
          (`SocialComponent.AddMembersToGroup` (`self.BP_Social`) _returnvalue_2 "INVESTIGATE" false))
        (:`Is Not Valid`
          (`SocialComponent.AddActorToGroup` (`self.BP_Social`) Ally "INVESTIGATE")))
      (`BlackboardComponent.SetValueAsVector` (`AIBlueprintHelperLibrary.GetBlackboard` null) "InvestigatePosition" (`BlackboardComponent.GetValueAsVector` (`AIBlueprintHelperLibrary.GetBlackboard` Ally) "InvestigatePosition")))))

(fn `OnLeaveInvestigation`
  (`BlackboardComponent.ClearValue` (`AIBlueprintHelperLibrary.GetBlackboard` null) "InvestigatePosition")
  (`SocialComponent.RemoveActorFromGroup` (`self.BP_Social`) self "INVESTIGATE"))

(fn `OnSawAllyChangedState`
  (params (Ally :type "Actor Object Reference") (NewState :type "EAlert Enum" :default "PASSIVE"))
  (locals (L_Ally :type "Actor Object Reference") (L_LineType :type "ELineType Enum") (L_PendingType :type "EPendingType Enum"))
  (bind _returnvalue (enumliteral `EPendingType` "INVALID"))
  (bind _bp_social (`self.BP_Social`))
  (bind _settings_maxinvestigators (break `SocialSettings` (`SocialComponent.Settings` _bp_social)))
  (bind _returnvalue_2 (`DialogueManager.GetLineTypePriority` (`DialogueComponent.DialogueManager` (`self.Dialogue`)) (`local.L_LineType`)))
  (bind _returnvalue_3 (`DialogueManager.HaveCommonActiveDialogue` (`DialogueComponent.DialogueManager` (`self.Dialogue`)) (`SocialComponent.GetMySocialGroup` (`self.BP_Social`)) (`SocialComponent.GetMySocialGroup` (`self.GetComponentByClass` (`local.L_Ally`) "/Game/AI/Components/BP_SocialComponent.BP_SocialComponent_C")) _returnvalue_2))
  (set `local.L_Ally` Ally)
  (bind (_canplay _alreadyplayingdialogue) (`/Game/AI/Components/BP_DialogueComponent.CanPlayADialogue` (`self.Dialogue`) NewState -1))
  (if _canplay
    (`DialogueComponent.ForgetDialogue` (`self.Dialogue`) _alreadyplayingdialogue true)
    (`|ExecutionSequence`
      (:`then_0`
        ; Try To find a line to play
        (switch `EAlert` NewState
          (:`PASSIVE`
            (switch `EAlert` (`SocialComponent.AlertState` (`self.BP_Social`))
              (:`PASSIVE`
                (set `local.L_LineType` "GREETING"))
              (:`INVESTIGATE`
                (if (< (`SocialComponent.GetSocialGroupSize` _bp_social) _settings_maxinvestigators) :!label _label
                  (set `local.L_LineType` "INVESTIGATION_MAIN")))
              (:`AGGRESSIVE_INVESTIGATE`
                (goto _label))))
          (:`INVESTIGATE`
            (switch `EAlert` (`SocialComponent.AlertState` (`self.BP_Social`))
              (:`PASSIVE`
                (set `local.L_LineType` "INVESTIGATION_SECONDARY")
                (set `local.L_PendingType` "ASK_TO_JOIN"))
              (:`INVESTIGATE`
                (if (> (`self.GetInvestigationPriority` self) (`self.GetInvestigationPriority` (`local.L_Ally`)))
                  _
                  (else
                    _))
                (set `local.L_LineType` "INVESTIGATION_BOTH_SECONDARY")
                (set `local.L_PendingType` "ASK_TO_JOIN"))))))
      (:`then_1`
        (if (!= (`local.L_LineType`) (`KismetMathLibrary.Conv_ByteToInt` (enumliteral `ELineType` "INVALID")))
          (if (not (`SocialComponent.ShouldIgnoreAnsweringLineType` (`self.BP_Social`) (`local.L_LineType`)))
            (bind (_canplay_2 _alreadyplayingdialogue_2) (`/Game/AI/Components/BP_DialogueComponent.CanPlayADialogue` (`self.GetComponentByClass` (`local.L_Ally`) "/Game/AI/Components/BP_DialogueComponent.BP_DialogueComponent_C") _returnvalue_2 -1))
            (if _canplay_2
              (if (not _returnvalue_3)
                (`/Game/AI/Components/BP_DialogueComponent.StartADialogue` (`self.Dialogue`) (`local.L_Ally`) (`local.L_LineType`) (`SocialComponent.GetSocialGroupSize` (`self.BP_Social`))))
              (elif (`DialogueManager.IsAMemberOfADialogue` (`DialogueComponent.DialogueManager` (`self.Dialogue`)) _alreadyplayingdialogue_2 self)
                _
                (elif (not _returnvalue_3)
                  ; Try to join a dialogue that can't be interrupted
                  (if (!= (`local.L_PendingType`) (`KismetMathLibrary.Conv_ByteToInt` _returnvalue))
                    (bind _returnvalue_4 (`DialogueManager.AddToPendingParticipants` (`DialogueComponent.DialogueManager` (`self.Dialogue`)) _alreadyplayingdialogue_2 self (`/Game/AI/Components/BP_DialogueComponent.GetSpeakPriority` (`self.Dialogue`) false (`self.K2_GetActorLocation` (`local.L_Ally`)) _returnvalue)))
                    (if _returnvalue_4
                      (`DialogueComponent.OnPendingToJoinDialogue` (`self.Dialogue`) _alreadyplayingdialogue_2 (`local.L_Ally`) (`local.L_PendingType`))
                      ; Debug
                      (`self.DebugOutput` "Can't interrupt dialogue %0, pending to join to AI %1" (`|MakeArray` (`KismetStringLibrary.Conv_IntToString` _alreadyplayingdialogue_2) (`KismetStringLibrary.Conv_IntToString` (`SocialComponent.GetID` (`self.GetComponentByClass` (`local.L_Ally`) "/Game/AI/Components/BP_SocialComponent.BP_SocialComponent_C"))))))))))))))
    (else
      (`self.DebugOutput` "Plays more important dialogue"))))

(fn `UserConstructionScript`)